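; Scene component that drives a targeting laser for pointing a fire weapon, using a Niagara beam and a target marker supplied through SetParameters.
; Each tick it pulses the beam colour's green channel and line-traces forward on Visibility to set the beam end.
; On a hit, it aligns the marker to the surface normal and scales it with distance.
; GetHitLocation exposes the latest result; the no-hit endpoint omits the start location.
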(event EventTick
  (params (DeltaSeconds :type Float%20%28single-precision%29))
  (bind _returnvalue (Utilities|Time|GetTimeSeconds))
  (bind _returnvalue_2 (Transformation|GetWorldLocation))
  (bind _returnvalue_3 (Math|Vector|GetForwardVector))
  (bind _target (Variables|Default|GetTarget))
  (bind _laserdistance (Variables|Default|GetLaserDistance))
  (bind _returnvalue_4 (Math|Trig|Sin(Radians) _returnvalue))
  (bind _returnvalue_5 (* _returnvalue_3 _laserdistance))
  (bind _output_get (Variables|Default|SetLaserColor (Utilities|Struct|MakeLinearColor (.r (Variables|Default|GetLaserColor)) (/ (* _returnvalue_4 _returnvalue_4) 1e+01) (.b (Variables|Default|GetLaserColor)) (.a (Variables|Default|GetLaserColor)))))
  (Effects|Components|ParticleSystem|SetColorParameter (Variables|Default|GetNSLaserPointing) "ColorBeam" _output_get)
  (bind _outhit (Collision|LineTraceByChannel _returnvalue_2 (+ _returnvalue_2 _returnvalue_5) "TraceTypeQuery1" false 0 "None"))
  (Variables|Default|SetbBlockingHit (.bblockinghit _outhit))
  (Variables|Default|SetTargetDistance (.distance _outhit))
  (bind _output_get_2 (Variables|Default|SetBlockingHitLocation (select (.bblockinghit _outhit) (.location _outhit) _returnvalue_5)))
  (Effects|Components|ParticleSystem|SetVectorParameter (Variables|Default|GetNSLaserPointing) "LaserEnd" _output_get_2)
  (Rendering|SetVisibility (Variables|Default|GetbBlockingHit) false)
  (if (Variables|Default|GetbBlockingHit)
    (Transformation|SetWorldLocation _target _output_get_2 false false)
    (Transformation|SetWorldRotation _target (Math|Conversions|RotationFromXVector (.impactnormal _outhit)) false false)
    (Transformation|SetRelativeScale3D _target (Math|Vector|MakeVector (* (Variables|Default|GetProportionScaleForDistance) (Variables|Default|GetTargetDistance)) (* (Variables|Default|GetProportionScaleForDistance) (Variables|Default|GetTargetDistance)) (* (Variables|Default|GetProportionScaleForDistance) (Variables|Default|GetTargetDistance))))))

(fn SetParameters
  (params (NSLaserPointing :type Niagara%20Component%20Object%20Reference) (Target :type Decal%20Component%20Object%20Reference) (LaserDistance :type Float%20%28single-precision%29))
  (Variables|Default|SetNSLaserPointing NSLaserPointing)
  (Variables|Default|SetTarget Target)
  (Variables|Default|SetLaserDistance LaserDistance))

(fn GetHitLocation
  (return (Variables|Default|GetbBlockingHit) (Variables|Default|GetBlockingHitLocation)))