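; BP_TurretControls is a turret weapon that sets up its FireWeapon component with pistol ammo, effects and sound, and projects an aiming laser.
; Each tick, a visibility line trace from LaserAiming sets the Niagara beam's end and the impact effect's position, showing the impact only on a hit.
; A squared time-based sine subtly pulses both effects' color.
; On a miss, the endpoint omits the laser's start location.
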(event EventBeginPlay
  (Class|FireWeaponComponent|SetWeaponandAmmo (Variables|Default|GetFireWeapon) "/Game/SciFiWeapLight/FX/Particles/P_Pistol_MuzzleFlash_Light.P_Pistol_MuzzleFlash_Light" "/Game/Game/GrabObjects/FireWeapon/SciFiPistolAmmo.SciFiPistolAmmo_C" "/Game/MilitaryWeapDark/Sound/Pistol/Wavs/PistolB_Fire01.PistolB_Fire01" "Muzzle" 0.2))

(event EventTick
  (params (DeltaSeconds :type Float%20%28single-precision%29))
  (bind _returnvalue (Utilities|Time|GetTimeSeconds))
  (bind _laseraiming (Variables|Default|GetLaserAiming))
  (bind _laserdistance (Variables|Default|GetLaserDistance))
  (bind _nslaserimpact (Variables|Default|GetNSLaserImpact))
  (bind _returnvalue_2 (Math|Trig|Sin(Radians) _returnvalue))
  (bind _returnvalue_3 (Transformation|GetWorldLocation _laseraiming))
  (bind _returnvalue_4 (Math|Vector|GetForwardVector _laseraiming))
  (bind _returnvalue_5 (* _returnvalue_4 _laserdistance))
  (bind _output_get (Variables|Default|SetLaserColor (Utilities|Struct|MakeLinearColor 1.0 (/ (* _returnvalue_2 _returnvalue_2) 1e+01) 0.0 0.5)))
  (Effects|Components|ParticleSystem|SetColorParameter (Variables|Default|GetNSLaserPointing) "ColorBeam" _output_get)
  (Effects|Components|ParticleSystem|SetColorParameter (Variables|Default|GetNSLaserImpact) "ColorImpact" _output_get)
  (bind _outhit (Collision|LineTraceByChannel _returnvalue_3 (+ _returnvalue_3 _returnvalue_5) "TraceTypeQuery1" false 0 "None"))
  (Effects|Components|ParticleSystem|SetVectorParameter (Variables|Default|GetNSLaserPointing) "LaserEnd" (select (.bblockinghit _outhit) (.location _outhit) _returnvalue_5))
  (Transformation|SetWorldLocation _nslaserimpact (select (.bblockinghit _outhit) (.location _outhit) _returnvalue_5) false false)
  (Rendering|SetVisibility _nslaserimpact (.bblockinghit _outhit) false))

(fn ConstructionScript)