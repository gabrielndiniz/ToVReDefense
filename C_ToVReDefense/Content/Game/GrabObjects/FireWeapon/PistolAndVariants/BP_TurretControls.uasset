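; BP_TurretControls is a grabbable turret control that fires SciFi pistol ammo and carries a pointing laser.
; On BeginPlay it configures the FireWeapon and PointingLaser components, caches the skeletal mesh's initial relative transform and binds to grab changes.
; Grabbing clears the mesh's constraint mode and stops the timeline.
; Releasing plays the timeline, which lerps the mesh toward the cached transform through a world-space teleport and sets the constraint mode to Default.
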(event Custom|ChangeGrab_Event
  (bind _skeletalmesh (Variables|Default|GetSkeletalMesh))
  (bind _returnvalue (Transformation|GetRelativeTransform _skeletalmesh))
  (if (Default|GetIsHeld (Variables|Default|GetGrabComponentSnap))
    (Class|PrimitiveComponent|SetConstraintMode (Variables|Default|GetSkeletalMesh) "None")
    (Variables|Default|SetAlpha 0.0)
    (bind _alphavalue (Timeline|Timeline_Alfa Stop)
      (:Update
        (Variables|Default|SetAlpha _alphavalue)
        (Transformation|SetWorldLocationAndRotation (Variables|Default|GetSkeletalMesh) (Math|Vector|Lerp(Vector) (.location _returnvalue) (Variables|Default|GetInitialLocation) (Variables|Default|GetAlpha)) (Math|Rotator|Lerp(Rotator) (.rotation _returnvalue) (Variables|Default|GetInitialRotation) (Variables|Default|GetAlpha) true) false true)
        (Class|PrimitiveComponent|SetConstraintMode (Variables|Default|GetSkeletalMesh) "Default")))
    (else
      (Timeline|Timeline_Alfa PlayFromStart))))

(event EventBeginPlay
  (bind _skeletalmesh (Variables|Default|GetSkeletalMesh))
  (bind _returnvalue (Transformation|GetRelativeTransform _skeletalmesh))
  (Class|FireWeaponComponent|SetWeaponandAmmo (Variables|Default|GetFireWeapon) "/Game/SciFiWeapLight/FX/Particles/P_Pistol_MuzzleFlash_Light.P_Pistol_MuzzleFlash_Light" "/Game/Game/GrabObjects/FireWeapon/PistolAndVariants/SciFiPistolAmmo.SciFiPistolAmmo_C" "/Game/MilitaryWeapDark/Sound/Pistol/Wavs/PistolB_Fire01.PistolB_Fire01" "Muzzle" 0.2)
  (Default|SetParameters (Variables|Default|GetPointingLaser) (Variables|Default|GetNSLaserPointing) (Variables|Default|GetNSLaserImpact) 5e+03)
  (Variables|Default|SetInitialLocation (.location _returnvalue))
  (Variables|Default|SetInitialRotation (.rotation _returnvalue))
  (EventDispatchers|AssignChangeGrab (delegate Custom|ChangeGrab_Event)))

(fn ConstructionScript)

(fn IsRightTurret
  (params (bIsRightTurret :type Boolean)))