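; BP_PistolAmmo is the projectile for the pistol.
; On BeginPlay it passes its mesh, movement, launch and impact blasts, explosion force, impact sound and tuning values to SetProjectile.
; It then enables query and physics collision on the Ammo mesh after a tiny delay inversely proportional to speed, meant to keep the shot from hitting the weapon.
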(event EventBeginPlay
  (Class|Projectile|SetProjectile (Variables|Default|GetAmmo) (Variables|Default|GetProjectileMovementComponent) (Variables|Default|GetLaunchBlastComponent) (Variables|Default|GetImpactBlastComponent) (Variables|Default|GetExplosionForceComponent) (Variables|Default|GetImpact%20Sound) 0.01 0.001 0.0 (Variables|Default|GetNew%20Speed) 1e+01)
  ;[1 1 1] It will activate collision after 20 units of distance, to garantee not shoot in the weapon
  (Utilities|FlowControl|Delay (/ 1e-05 (Variables|Default|GetNew%20Speed)))
  (Collision|SetCollisionEnabled (Variables|Default|GetAmmo) "QueryAndPhysics"))

(fn ConstructionScript)