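; Grabbable laser marker in the pistol family, with a pointing laser, a widget interactor and a turret burst effect.
; Construction sets up the burst effect, and BeginPlay wires the pointer and laser, then caches the mesh's initial transform and widget scale.
; Grabbing clears the mesh's constraint mode and hides the widget by zeroing its scale.
; Releasing restores the widget and runs a timeline that lerps the mesh toward its initial transform, setting the default constraint mode.
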(event Custom|ChangeGrab_Event
  (bind _skeletalmesh (Variables|Default|GetSkeletalMesh))
  (bind _returnvalue (Transformation|GetRelativeTransform _skeletalmesh))
  ;[1 1 1] In case of released, goes back to place.
  (if (Default|GetIsHeld (Variables|Default|GetGrabComponentSnap))
    (Class|PrimitiveComponent|SetConstraintMode (Variables|Default|GetSkeletalMesh) "None")
    (Variables|Default|SetAlpha 0.0)
    (Transformation|SetRelativeScale3D (Variables|Default|GetWidget) "0, 0, 0")
    (bind _alphavalue (Timeline|Timeline_0 Stop)
      (:Update
        (Variables|Default|SetAlpha _alphavalue)
        (Transformation|SetWorldLocationAndRotation (Variables|Default|GetSkeletalMesh) (Math|Vector|Lerp(Vector) (.location _returnvalue) (Variables|Default|GetInitialLocation) (Variables|Default|GetAlpha)) (Math|Rotator|Lerp(Rotator) (.rotation _returnvalue) (Variables|Default|GetInitialRotation) (Variables|Default|GetAlpha) true) false true)
        (Class|PrimitiveComponent|SetConstraintMode (Variables|Default|GetSkeletalMesh) "Default")))
    (else
      (Transformation|SetRelativeScale3D (Variables|Default|GetWidget) (Variables|Default|GetWidgetScale))
      (Timeline|Timeline_0 PlayFromStart))))

(event EventBeginPlay
  (bind _skeletalmesh (Variables|Default|GetSkeletalMesh))
  (bind _returnvalue (Transformation|GetRelativeTransform _skeletalmesh))
  (Class|WidgetInteractorComponent|SetPointer (Variables|Default|GetWidgetInteractor) (Variables|Default|GetPointer))
  (Default|SetParameters (Variables|Default|GetPointingLaser) (Variables|Default|GetNSLaserPointing) (Variables|Default|GetNSLaserImpact) 1e+04)
  (Variables|Default|SetInitialLocation (.location _returnvalue))
  (Variables|Default|SetInitialRotation (.rotation _returnvalue))
  (Variables|Default|SetWidgetScale (Transformation|GetWorldScale (Variables|Default|GetWidget)))
  (EventDispatchers|AssignChangeGrab (delegate Custom|ChangeGrab_Event)))

(event EventTick
  (params (DeltaSeconds :type Float%20%28single-precision%29)))

(fn ConstructionScript
  (Default|SetParameters (Variables|Default|GetBurst) (Variables|Default|GetNS_TurretBurst)))