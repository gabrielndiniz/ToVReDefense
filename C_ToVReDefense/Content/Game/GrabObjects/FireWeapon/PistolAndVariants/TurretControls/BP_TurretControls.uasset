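; Grabbable turret controls that aim a turret-mode FireWeapon, with the turret sphere offset sideways by hand.
; Each tick, FireWeapon points using hit results from a pointing laser and a longer-range targeting laser.
; Grab changes toggle the GuidanceSystem constraint, and on release a timeline lerps it back toward its initial transform.
; Construction configures the targeting laser, anti-gravity and turret burst effects.
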(event Custom|ChangeGrab_Event
  (bind _guidance_system (Variables|Default|GetGuidance%20System))
  (bind _returnvalue (Transformation|GetRelativeTransform _guidance_system))
  ;[1 1 1] In case of released, goes back to place.
  (if (Default|GetIsHeld (Variables|Default|GetGrabComponentSnap))
    (Class|PrimitiveComponent|SetConstraintMode (Variables|Default|GetGuidance%20System) "None")
    (Variables|Default|SetAlpha 0.0)
    (bind _alphavalue (Timeline|Timeline_Alfa Stop)
      (:Update
        (Variables|Default|SetAlpha _alphavalue)
        (Transformation|SetWorldLocationAndRotation (Variables|Default|GetGuidance%20System) (Math|Vector|Lerp(Vector) (.location _returnvalue) (Variables|Default|GetInitialLocation) (Variables|Default|GetAlpha)) (Math|Rotator|Lerp(Rotator) (.rotation _returnvalue) (Variables|Default|GetInitialRotation) (Variables|Default|GetAlpha) true) false true)
        (Class|PrimitiveComponent|SetConstraintMode (Variables|Default|GetGuidance%20System) "Default")))
    (else
      (Timeline|Timeline_Alfa PlayFromStart))))

(event EventBeginPlay
  (bind _guidance_system (Variables|Default|GetGuidance%20System))
  (bind _returnvalue (Transformation|GetRelativeTransform _guidance_system))
  ;[1 1 1] Setting Components
  (Class|FireWeaponComponent|SetWeaponandAmmo (Variables|Default|GetFireWeapon) (Variables|Default|GetNew%20Muzzle%20Flash) (Variables|Default|GetNew%20Projectile%20Classes) (Variables|Default|GetNew%20Fire%20Sound) (Variables|Default|GetMuzzle) (Variables|Default|GetNew%20Callback%20Time) true (Variables|Default|GetSphere))
  (Default|SetParameters (Variables|Default|GetPointingLaser) (Variables|Default|GetNSLaserPointing) (Variables|Default|GetNSLaserImpact) 5e+03)
  (Variables|Default|SetInitialLocation (.location _returnvalue))
  (Variables|Default|SetInitialRotation (.rotation _returnvalue))
  (EventDispatchers|AssignChangeGrab (delegate Custom|ChangeGrab_Event)))

(event EventTick
  (params (DeltaSeconds :type Float%20%28single-precision%29))
  (bind _targetinglaser (Variables|Default|GetTargetingLaser))
  (bind (_bithit _location) (Default|GetHitLocation _targetinglaser))
  ;[1 1 1] Rotate the turret
  (Class|FireWeaponComponent|PointatTarget (Variables|Default|GetFireWeapon) (.Location (Default|GetHitLocation (Variables|Default|GetPointingLaser))) _location _bithit))

(fn ConstructionScript
  (Default|SetParameters (Variables|Default|GetTargetingLaser) (Variables|Default|GetNSLaserPointing1) (Variables|Default|GetDecal) 5e+04)
  (Default|SetParameters (Variables|Default|GetAntiGravity) (Variables|Default|GetNSAntiGravity))
  (Default|SetParameters (Variables|Default|GetTurretBurst) (Variables|Default|GetNS_TurretBurst))
  (if (Class|Grabbable|GetIsforRightHand)
    (Transformation|AddRelativeLocation (Variables|Default|GetSphere) (Math|Vector|MakeVector (* (Variables|Default|GetHorizontalDistance) -1.0) 0.0 0.0) false false)
    (else
      (Transformation|AddRelativeLocation (Variables|Default|GetSphere) (Math|Vector|MakeVector (Variables|Default|GetHorizontalDistance) 0.0 0.0) false false))))