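; Player cockpit Blueprint that shows health as a screen color and keeps a death count.
; On BeginPlay it creates a dynamic material for one slot of the WireFrame mesh and caches max health from Health.
; Every Tick it blends that material's Color from dim green at full health to dim red at zero.
; Separate functions increment and return the death count, independent of the display.
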(event EventTick
  (params (DeltaSeconds :type Float%20%28single-precision%29))
  (bind _health (Variables|Default|GetHealth))
  (bind _maxhealth (Variables|Default|GetMaxHealth))
  (bind _returnvalue (Class|HealthComponent|GetHealth _health))
  (bind _returnvalue_2 (/ _returnvalue _maxhealth))
  (bind _returnvalue_3 (* _returnvalue_2 0.1))
  (Rendering|Material|SetVectorParameterValue (Variables|Default|GetHealthScreenMaterial) "Color" (Utilities|Struct|MakeLinearColor (* -1 (- _returnvalue_3 0.1)) _returnvalue_3 0.0 1.0) :!class /Script/Engine.MaterialInstanceDynamic))

(event EventBeginPlay
  (bind _returnvalue (Rendering|Material|CreateDynamicMaterialInstance (Variables|Default|GetWireFrame) 3 "/Game/Game/Character/Player/UIScreen_Placeholder_e_D_Mat_Health.UIScreen_Placeholder_e_D_Mat_Health" "None" :!class /Script/Engine.PrimitiveComponent))
  (Variables|Default|SetHealthScreenMaterial _returnvalue)
  (Variables|Default|SetMaxHealth (Class|HealthComponent|GetMaxHealth (Variables|Default|GetHealth))))

(fn ConstructionScript)

(fn AddDeathCount
  (Variables|Default|SetCurrentDeathCount (+ (Variables|Default|GetCurrentDeathCount) 1)))

(fn GetDeathCount
  (return (Variables|Default|GetCurrentDeathCount)))