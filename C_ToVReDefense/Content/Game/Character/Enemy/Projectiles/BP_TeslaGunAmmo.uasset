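; BP_TeslaGunAmmo is an enemy Tesla gun projectile with impact blast, explosion force and sound.
; BeginPlay passes its components and damage, speed and destroy settings to SetProjectile, then enables Ammo collision after a tiny speed-derived delay meant to avoid hitting the firing weapon.
; Tick stretches the launch blast effect in proportion to speed up to a cap, offsetting it as it grows to form a lengthening bolt.
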(event EventBeginPlay
  (Class|Projectile|SetProjectile (Variables|Default|GetAmmo) (Variables|Default|GetProjectileMovementComponent) (Variables|Default|GetLaunchBlastComponent) (Variables|Default|GetImpactBlastComponent) (Variables|Default|GetExplosionForceComponent) (Variables|Default|GetImpact%20Sound) 1.0 4e+01 0.0 (Variables|Default|GetNew%20Speed) 1e+01)
  ;[1 1 1] It will activate collision after 20 units of distance, to garantee not shoot in the weapon
  (Utilities|FlowControl|Delay (/ 0.0001 (Variables|Default|GetNew%20Speed)))
  (Collision|SetCollisionEnabled (Variables|Default|GetAmmo) "QueryAndPhysics"))

(event EventTick
  (params (DeltaSeconds :type Float%20%28single-precision%29))
  (if (< (Variables|Default|GetXScale) 1e+02)
    (Variables|Default|SetXScale (+ (* DeltaSeconds (Variables|Default|GetNew%20Speed) 0.166) (Variables|Default|GetXScale)))
    (Transformation|SetRelativeTransform (Variables|Default|GetLaunchBlastComponent) (Math|Transform|MakeTransform (Math|Vector|MakeVector (* (Variables|Default|GetScaleLocationRelation) (Variables|Default|GetXScale)) 0.0 0.0) "0,90.000000, 0" (Math|Vector|MakeVector 5e+01 (Variables|Default|GetXScale) 5e+01)) false false)))

(fn ConstructionScript)