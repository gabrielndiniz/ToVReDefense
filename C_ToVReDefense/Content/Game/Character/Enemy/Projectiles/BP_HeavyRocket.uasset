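; BP_HeavyRocket is an enemy heavy rocket projectile with area damage and explosion force.
; On BeginPlay it passes its Ammo mesh, movement, launch and impact blasts, explosion force and tuning values to SetProjectile.
; It then enables Ammo collision after a tiny speed-scaled delay, intended to keep it from hitting the firing weapon.
; SetMaterial swaps the mesh's second material slot.
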(event EventBeginPlay
  (Class|Projectile|SetProjectile (Variables|Default|GetAmmo) (Variables|Default|GetProjectileMovementComponent) (Variables|Default|GetLaunchBlastComponent) (Variables|Default|GetImpactBlastComponent) (Variables|Default|GetExplosionForceComponent) 0.01 6e+01 1e+02 (Variables|Default|GetNew%20Speed) 1e+02)
  ;[1 1 1] It will activate collision after 20 units of distance, to garantee not shoot in the weapon
  (Utilities|FlowControl|Delay (/ 0.0001 (Variables|Default|GetNew%20Speed)))
  (Collision|SetCollisionEnabled (Variables|Default|GetAmmo) "QueryAndPhysics"))

(fn ConstructionScript)

(fn SetMaterial
  (params (Material :type Material%20Interface%20Object%20Reference))
  (Rendering|Material|SetMaterial (Variables|Default|GetAmmo) 1 Material))