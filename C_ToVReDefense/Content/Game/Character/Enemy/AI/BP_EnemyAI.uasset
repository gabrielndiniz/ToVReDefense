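; BP_EnemyAI is an enemy AI controller that starts behavior tree logic when it possesses a pawn and stops it on unpossess.
; For BP_mainRobotPart pawns it sets up the BCAIRobotDriver component, which is destroyed for other pawn types and stopped on unpossess.
; A floating pawn movement component is added to robots solely to switch navigation agents.
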(event EventUnPossess
  (params (UnpossessedPawn :type Pawn%20Object%20Reference))
  (Default|Stop (Variables|Default|GetBC_AIRobotDriver) false)
  (AI|Logic|StopLogic (Variables|Default|GetBehaviorTree) ""))

(event EventPossess
  (params (PossessedPawn :type Pawn%20Object%20Reference))
  ;[1 1 1] Setup robot driver component
  (bind _asbp_main_robot_part (Utilities|Casting|CastToBP_mainRobotPart PossessedPawn)
    (:then
      (Variables|Default|SetMyRobot _asbp_main_robot_part)
      (AddComponent|AddFloatingPawnMovement (Variables|Default|GetMyRobot)) ; Warning! This floating pawn movement component is \nONLY used for switching navigation agents for the robot
      (Default|Setup (Variables|Default|GetBC_AIRobotDriver) (Variables|Default|GetMyRobot))
      (AI|Logic|StartLogic (Variables|Default|GetBehaviorTree)))
    (:CastFailed
      (Components|DestroyComponent (Variables|Default|GetBC_AIRobotDriver))
      (AI|Logic|StartLogic (Variables|Default|GetBehaviorTree)))))

(fn ConstructionScript)