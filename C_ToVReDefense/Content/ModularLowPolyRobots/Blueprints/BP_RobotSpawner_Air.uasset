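; BP_RobotSpawner_Air is a spawner child Blueprint that randomizes the build of a modular low-poly air robot.
; On BeginPlay it passes a random body type, chassis, two independently picked guns and a color from its arrays to Config.
; It then calls the parent BeginPlay, so the random setup is applied before the inherited logic runs.
; The construction script only calls the parent version.
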(event EventBeginPlay
  (CallFunction|Config (.OutItem (Utilities|Array|Random (Variables|Default|GetBody%20Types))) (.OutItem (Utilities|Array|Random (Variables|Default|GetChassis))) (Utilities|Array|MakeArray (.OutItem (Utilities|Array|Random (Variables|Default|GetGuns))) (.OutItem (Utilities|Array|Random (Variables|Default|GetGuns)))) (.OutItem (Utilities|Array|Random (Variables|Default|GetColors_0))))
  (|CallParentFunction))

(fn ConstructionScript
  (|CallParentFunction))